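; Melee enemy AI that chases the player on sight, punches, and dies when its health runs out.
; PawnSensing triggers an AI MoveTo; arrival starts a delayed attack with a distance-checked hit, then a cooldown that blocks new moves.
; Taking damage updates an overhead health bar, turned toward the player camera every Tick, and either restarts pursuit when not attacking or triggers death and destruction.
; Animations play directly on the mesh.
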(event OnSeePawn(PawnSensing)
  (params (Pawn :type Pawn%20Object%20Reference))
  ;[1 1 1] On See Pawn
  (Utilities|Casting|CastToThirdPersonCharacter Pawn)
  (CallFunction|GotoPlayer))

(event Custom|Take%20Damage
  (params (NewParam :type Float%20%28single-precision%29))
  ;[1 1 1] Take Damage
  (if (not (Variables|Default|GetisDead))
    (bind _output_get (Variables|Default|Sethealth (- (Variables|Default|Gethealth) NewParam)))
    (Progress|SetPercent (Variables|/Game/M_Asset/Widgets/enemyUI.enemyUI_C|GetProgressBar_0 (Variables|Default|GetAs%20Enemy%20UI)) (/ (Variables|Default|GetHealth) (Variables|Default|GethealthMax)))
    (if (<= _output_get 0.0)
      (Variables|Default|SetisDead true)
      (Components|Animation|PlayAnimation (Variables|Character|GetMesh) "/Game/M_Asset/Anim/Dying_Backwards.Dying_Backwards" false)
      (Utilities|FlowControl|Delay 4.0)
      (Actor|DestroyActor)
      (elif (not (Variables|Default|GetisAttack))
        (CallFunction|GotoPlayer)))))

(event Custom|Cooldown
  ;[1 1 1] Cooldown
  (Variables|Default|SetcanMove false)
  (Utilities|FlowControl|Delay (Variables|Default|GetcooldownAttack))
  (Variables|Default|SetcanAttack true)
  (Variables|Default|SetisAttack false)
  (if (not (Variables|Default|GetisDead))
    (Components|Animation|PlayAnimation (Variables|Character|GetMesh) "/Game/M_Asset/Anim/Idle.Idle" true)
    (Utilities|FlowControl|Delay 1.0)
    (Variables|Default|SetcanMove true)))

(event Custom|GotoPlayer
  ;[1 1 1] Go to Player
  (if (not (Variables|Default|GetisDead))
    (if (Variables|Default|GetcanMove)
      (AI|AIMoveTo self "0, 0, 0" (Game|GetPlayerCharacter 0) 6e+01 false
        (:then
          (Utilities|FlowControl|DoOnce false :!label _label
            (:Completed
              (Components|Animation|PlayAnimation (Variables|Character|GetMesh) "/Game/M_Asset/Anim/Crouch_Walk_Forward.Crouch_Walk_Forward" true))))
        (:OnSuccess
          (CallFunction|Attack)
          (goto _label Reset))))))

(event Custom|Attack
  ;[1 1 1] Attack
  (if (not (Variables|Default|GetisDead))
    (Utilities|FlowControl|Delay 0.5)
    (Variables|Default|SetisAttack true)
    (Components|Animation|PlayAnimation (Variables|Character|GetMesh) "/Game/M_Asset/Anim/Punching_Anim_mixamo_com.Punching_Anim_mixamo_com" false)
    (CallFunction|Cooldown)
    (if (< (Math|Vector|Distance(Vector) (Transformation|GetActorLocation) (Transformation|GetActorLocation (Variables|Default|GetAs%20Third%20Person%20Character))) 1.5e+02)
      (Default|TakeDamage (Variables|Default|GetAs%20Third%20Person%20Character) (Variables|Default|GetDamage)))))

(event EventBeginPlay
  ;[1 1 1] BeginPlay
  (Utilities|FlowControl|Sequence
    (:then_0
      (Variables|Default|Sethealth (Variables|Default|GethealthMax))
      (bind _asthird_person_character (Utilities|Casting|CastToThirdPersonCharacter (Game|Player|GetPlayerPawn 0)))
      (Variables|Default|SetAs%20Third%20Person%20Character _asthird_person_character)
      (bind _asenemy_ui (Utilities|Casting|CastToenemyUI (UserInterface|GetWidget (Variables|Default|GetWidget))))
      (bind _output_get (Variables|Default|SetAs%20Enemy%20UI _asenemy_ui))
      (Progress|SetPercent (Variables|/Game/M_Asset/Widgets/enemyUI.enemyUI_C|GetProgressBar_0 _output_get) (/ (Variables|Default|GetHealth) (Variables|Default|GethealthMax))))
    (:then_1
      (Components|Animation|PlayAnimation (Variables|Character|GetMesh) "/Game/M_Asset/Anim/Idle.Idle" true))))

(event EventTick
  (params (DeltaSeconds :type Float%20%28single-precision%29))
  ;[1 1 1] Tick
  (Transformation|SetWorldRotation (Variables|Default|GetWidget) (Math|Rotator|FindLookatRotation (Transformation|GetWorldLocation (Variables|Default|GetWidget)) (Transformation|GetWorldLocation (Variables|/Game/M_Asset/Blueprints/ThirdPersonCharacter.ThirdPersonCharacter_C|GetFollowCamera (Variables|Default|GetAs%20Third%20Person%20Character)))) false false))

(fn ConstructionScript)